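; WeaponConfig is a lookup asset that resolves weapon classes and ammo crate visuals from a weapon enum or ID.
; Classes come from the Weapons collection by ID, and the enum lookup converts its value to an integer index, so enum order must match that collection.
; GetWeaponAmmoMesh switches on the enum for Skorpion and Blaster, returning assets that are named as materials despite the function name.
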(fn GetWeaponClass
  (params (id :type Integer))
  (return (Utilities|Array|Get(acopy) (LocalVariables|GetWeapons) id)))

(fn GetWeaponfromEnum
  (params (weaponEnum :type WeaponList%20Enum))
  (return (CallFunction|GetWeaponClass (Math|Conversions|ToInteger(Byte) weaponEnum))))

(fn GetWeaponAmmoMesh
  (params (weaponEnum :type WeaponList%20Enum))
  (switch Utilities|FlowControl|Switch|SwitchonWeaponList weaponEnum
    (:NewEnumerator0
      (return "/Game/Assets/GameObjects/crates/ammo_create_1_Mat.ammo_create_1_Mat"))
    (:NewEnumerator1
      (return "/Game/Assets/GameObjects/crates/ammo_crate_2_Mat.ammo_crate_2_Mat"))))