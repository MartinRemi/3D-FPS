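; Bullet actor that damages what it hits, then destroys itself.
; The game instance's FriendlyFireOn flag sets who is spared: only the shooter when on, or CharacterBP teammates of the shooter when off.
; After applying damage, the ManageKillCollapse graph checks whether a hit PlayerBP has no health left, then records a kill on the shooter's PlayerStateBP and a death on the victim's.
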(event EventBeginPlay
  (bind _asthird_person_game_instane (Utilities|Casting|CastToThirdPersonGameInstane (Game|GetGameInstance)))
  (Variables|Default|SetgameInstance _asthird_person_game_instane))

(event EventActorBeginOverlap
  (params (OtherActor :type Actor%20Object%20Reference)))

(event EventTick
  (params (DeltaSeconds :type Float%20%28single-precision%29)))

(event Collision|EventHit
  (params (MyComp :type Primitive%20Component%20Object%20Reference) (Other :type Actor%20Object%20Reference) (OtherComp :type Primitive%20Component%20Object%20Reference) (bSelfMoved :type Boolean) (HitLocation :type Vector :default "0, 0, 0") (HitNormal :type Vector :default "0, 0, 0") (NormalImpulse :type Vector :default "0, 0, 0") (Hit :type Hit%20Result%20Structure%20%28by%20ref%29))
  (bind _returnvalue (Game|GetInstigatorController))
  ;[1 1 1] apply damages
  (if (Variables|/Game/Blueprints/ThirdPersonGameInstane.ThirdPersonGameInstane_C|GetfriendlyFireOn (Variables|Default|GetgameInstance))
    (if (== Other (Game|GetInstigator))
      (Actor|DestroyActor :!label _label)
      (else
        (Game|Damage|ApplyDamage Other (Variables|Default|GetDamages) _returnvalue self :!label _label_2)
        (Utilities|FlowControl|Sequence
          (:then_0
            (|ManageKillCollapse Other _returnvalue))
          (:then_1
            (goto _label)))))
    (else
      (bind _ascharacter_bp (Utilities|Casting|CastToCharacterBP Other)
        (:then
          (bind _ascharacter_bp_2 (Utilities|Casting|CastToCharacterBP (Game|GetInstigator))
            (:then
              (if (== (Variables|/Game/Blueprints/CharacterBP.CharacterBP_C|Getteam _ascharacter_bp_2) (Variables|/Game/Blueprints/CharacterBP.CharacterBP_C|Getteam _ascharacter_bp))
                (goto _label)
                (else
                  (goto _label_2))))
            (:CastFailed
              (goto _label_2))))
        (:CastFailed
          (goto _label_2))))))

(fn ConstructionScript)