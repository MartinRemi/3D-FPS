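; CharacterBP is a character Blueprint that handles damage, health and a simple timed respawn.
; AnyDamage lowers Health while Damageable is set, and at zero waits briefly before calling Respawn on the authority.
; If Respawnable, Respawn hides the actor and disables collision for a fixed delay, then restores both without resetting Health.
; OnRep_health caps Health at MaxHealth and notifies the HUD assigned through sethud.
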(event Custom|Respawn
  (params (Actor :type Actor%20Object%20Reference) (controller :type Controller%20Object%20Reference))
  (if (Variables|Default|Getrespawnable)
    (Collision|SetActorEnableCollision false)
    (Rendering|SetActorHiddenInGame true)
    (Utilities|FlowControl|Delay 2e+01)
    (Rendering|SetActorHiddenInGame false)
    (Collision|SetActorEnableCollision true)))

(event Custom|Event%20set%20hud
  (params (new%20hud :type Player%20Hud%20Object%20Reference))
  (Variables|Default|Sethud new%20hud))

(event EventActorBeginOverlap
  (params (OtherActor :type Actor%20Object%20Reference)))

(event Game|Damage|EventAnyDamage
  (params (Damage :type Float%20%28single-precision%29) (DamageType :type Damage%20Type%20Object%20Reference) (InstigatedBy :type Controller%20Object%20Reference) (DamageCauser :type Actor%20Object%20Reference))
  ;[1 1 1] Damage managment
  (if (Variables|Default|Getdamageable)
    (Development|PrintString (Utilities|String|Append "HIT " (Utilities|GetDisplayName self)) true true "(R=0.936703,G=0.342049,B=1.000000,A=1.000000)" 1e+01)
    (Variables|Default|Sethealth (- (Variables|Default|Gethealth) Damage))
    (if (<= (Variables|Default|Gethealth) 0.0)
      ;;[1 1 1] there should be an animation
      (Utilities|FlowControl|Delay 0.2)
      (Networking|SwitchHasAuthority
        (:Authority
          (CallFunction|Respawn self (Pawn|GetController)))))))

(fn ConstructionScript)

(fn OnRepHealth
  (bind _max_health (Variables|Default|Getmax_health))
  (bind _hud (Variables|Default|Gethud))
  (if (> (Variables|Default|Gethealth) _max_health)
    (Variables|Default|Sethealth _max_health))
  (if (Utilities|IsValid _hud)
    (Default|EventHealthChange _hud)))